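; BP_Line is a Blueprint that strings a cable between two referenced actors, PCH1 and PCH2.
; On BeginPlay it snaps a component to PCH1's root and attaches the Cable's end to PCH2's root.
; A calculation setting cable length to the distance between the two actors is present but never runs, and Tick and the construction script are empty.
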(event `self.ReceiveTick`
  (params (DeltaSeconds :type "Float (single-precision)")))

(event `self.ReceiveBeginPlay`
  (`self.K2_AttachToComponent` self (`Actor.RootComponent` (`self.PCH1`)) "None" "SnapToTarget" "SnapToTarget" "SnapToTarget" true)
  (`CableComponent.SetAttachEndToComponent` (`self.Cable`) (`Actor.RootComponent` (`self.PCH2`)) "None"))

(fn `UserConstructionScript`)