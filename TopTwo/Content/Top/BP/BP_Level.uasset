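; Level actor for a grid puzzle with red and blue starts, which also adds the UMG widget on BeginPlay.
; The construction script rebuilds cubes, walls, buttons and doors from config arrays, optionally randomizing default cube types and showing index labels.
; Helper functions look up components by index, grid position or ID, swap cube types, and color a target marker.
; Straight-line paths become index pairs, checked against walls and scale doors.
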(event `self.ReceiveBeginPlay`
  (bind _returnvalue (`|CreateWidget` (`self.UMG`) (`GameplayStatics.GetPlayerController` 0)))
  (`UserWidget.AddToViewport` _returnvalue 0))

(fn `FUN Check Distance`
  (params (IndexRow :type Integer) (IndexColumn :type Integer) (TargetRow :type Integer) (TargrtColumn :type Integer))
  (returns (Distance :type Integer))
  (return (- (+ (`KismetMathLibrary.Abs_Int` (- IndexRow TargetRow)) (`KismetMathLibrary.Abs_Int` (- IndexColumn TargrtColumn))) 1)))

(fn `FUN Check HaveWall`
  (params (AIndex :type Integer) (BIndex :type Integer))
  (returns (ReturnValue :type Boolean))
  (for _array_element (`self.BlockWall`)
    (bind (_a _b) (break `/Game/Top/BP/Variable/Str_BlockWall` _array_element))
    (if (or (and (== _a AIndex) (== _b BIndex)) (and (== _b AIndex) (== _a BIndex)))
      (return true)))
  (return false))

(fn `FUN Check Is Line`
  (params (IndexRow :type Integer) (IndexColumn :type Integer) (TargetRow :type Integer) (TargrtColumn :type Integer))
  (returns (Y :type Boolean) (Row :type Boolean))
  (bind _returnvalue (== IndexRow TargetRow))
  (return (or _returnvalue (== IndexColumn TargrtColumn)) _returnvalue))

(fn `FUN Check Path`
  (params (IndexRow :type Integer) (IndexColumn :type Integer) (TargetRow :type Integer) (TargrtColumn :type Integer))
  (returns (ReturnValue :type Boolean) (Path :type "Array of /Game/Top/BP/Variable/Str_BlockWall Structure"))
  (bind _path (`self.FUN_Get_Path` IndexRow IndexColumn TargetRow TargrtColumn))
  (for _array_element _path
    (bind (_a _b) (break `/Game/Top/BP/Variable/Str_BlockWall` _array_element))
    (bind _returnvalue (`self.FUN Check HaveWall` _a _b))
    (if _returnvalue
      (return false)))
  (return true _path))

(fn `FUN Check Scale`
  (params (Path :type "Array of /Game/Top/BP/Variable/Str_BlockWall Structure"))
  (returns (ReturnValue :type Boolean))
  (for _array_element Path
    (if (> (`KismetArrayLibrary.Array_Find` (`self.ScaleDoor`) (`.B_4_1D535E5A4D7EF1EADD184C9CD7FEA18C` (break `/Game/Top/BP/Variable/Str_BlockWall` _array_element))) -1)
      (return false)))
  (return true))

(fn `FUN_ClearCube`
  (locals (Local :type "Array of SceneComponent Object Reference"))
  (bind _output_get (set `local.Local` (`SceneComponent.GetChildrenComponents` (`self.Com_Cubes`) true)))
  (for _array_element _output_get
    (`ActorComponent.K2_DestroyComponent` _array_element))
  (`KismetArrayLibrary.Array_Clear` (`self.Cubes`)))

(fn `FUN_Compare_Size`
  (params (A :type Integer) (B :type Integer))
  (returns (Small :type Integer) (Large :type Integer) (ReturnValue :type Boolean))
  (bind _returnvalue (< A B))
  (return (select `bool` _returnvalue :`false` B :`true` A) (select `bool` _returnvalue :`false` A :`true` B) _returnvalue))

(fn `FUN_Get_Button_ByRow`
  (params (Row :type Integer) (Column :type Integer))
  (returns (IsValid :type Boolean) (`AsComs Button` :type "/Game/Top/BP/Coms_Button Object Reference"))
  (locals (NewLocalVar_2 :type Integer :default 0))
  (bind _output_get (set `local.NewLocalVar_2` (`/Game/Top/BP/Coms_Cube.Index` (`self.FUN_Get_Com_ByRow` Row Column))))
  (for _array_element (`SceneComponent.GetChildrenComponents` (`self.Com_Button`) true)
    (bind _ascoms_button (cast `/Game/Top/BP/Coms_Button` _array_element))
    (if (== (`/Game/Top/BP/Coms_Button.Index` _ascoms_button) _output_get)
      (return true _ascoms_button)))
  (return false null))

(fn `FUN_Get_Com_ByIndex`
  (params (Index :type Integer))
  (returns (Com :type "/Game/Top/BP/Coms_Cube Object Reference") (IsValid :type Boolean))
  (for _array_element (`self.Cubes`)
    (if (== (`/Game/Top/BP/Coms_Cube.Index` _array_element) Index)
      (return _array_element true)))
  (return null false))

(fn `FUN_Get_Com_ByRow`
  (params (Row :type Integer) (Column :type Integer))
  (returns (Com :type "/Game/Top/BP/Coms_Cube Object Reference"))
  (for _array_element (`self.Cubes`)
    (if (and (== (`/Game/Top/BP/Coms_Cube.IndexRow` _array_element) Row) (== (`/Game/Top/BP/Coms_Cube.IndexColumn` _array_element) Column))
      (return _array_element))))

(fn `FUN_Get_Door_ByID`
  (params (ID :type Integer))
  (returns (IsValid :type Boolean) (`AsComs Door` :type "/Game/Top/BP/Coms_Door Object Reference"))
  (for _array_element (`SceneComponent.GetChildrenComponents` (`self.Com_Door`) true)
    (bind _ascoms_door (cast `/Game/Top/BP/Coms_Door` _array_element))
    (if (== (`.ID_9_1D535E5A4D7EF1EADD184C9CD7FEA18C` (break `/Game/Top/BP/Variable/Str_Door` (`/Game/Top/BP/Coms_Door.Info` _ascoms_door))) ID)
      (return true _ascoms_door)))
  (return false null))

(fn `FUN_Get_DoorScale_ByIndex`
  (params (Index :type Integer))
  (returns (IsValid :type Boolean) (`AsComs Door Scale` :type "/Game/Top/BP/Coms_Door_Scale Object Reference"))
  (for _array_element (`SceneComponent.GetChildrenComponents` (`self.Com_Door`) true)
    (bind _ascoms_door_scale (cast `/Game/Top/BP/Coms_Door_Scale` _array_element))
    (if (== (`.IndexA_16_2FB6EDDC46584D5019EB2B9F084DBD42` (break `/Game/Top/BP/Variable/Str_Door` (`/Game/Top/BP/Coms_Door.Info` _ascoms_door_scale))) Index)
      (return true _ascoms_door_scale)))
  (return false null))

(fn `FUN_Get_Path`
  (params (IndexRow :type Integer) (IndexColumn :type Integer) (TargetRow :type Integer) (TargrtColumn :type Integer))
  (returns (Path :type "Array of /Game/Top/BP/Variable/Str_BlockWall Structure"))
  (locals (NewLocalVar_0 :type "Array of /Game/Top/BP/Variable/Str_BlockWall Structure") (NewLocalVar_1 :type Integer))
  (bind _newlocalvar_1 (`local.NewLocalVar_1`))
  (bind (_y _row) (`self.FUN Check Is Line` IndexRow IndexColumn TargetRow TargrtColumn))
  (if _y
    (bind (_small _large _returnvalue) (`self.FUN_Compare_Size` (`/Game/Top/BP/Coms_Cube.Index` (`self.FUN_Get_Com_ByRow` IndexRow IndexColumn)) (`/Game/Top/BP/Coms_Cube.Index` (`self.FUN_Get_Com_ByRow` TargetRow TargrtColumn))))
    (set `local.NewLocalVar_1` _small)
    (bind _returnvalue_2 (+ (`local.NewLocalVar_1`) (`KismetMathLibrary.SelectInt` 1 (`self.Column`) _row)))
    (`KismetArrayLibrary.Array_Add` (`local.NewLocalVar_0`) (make `/Game/Top/BP/Variable/Str_BlockWall` (select `bool` _returnvalue :`false` _returnvalue_2 :`true` _newlocalvar_1) (select `bool` _returnvalue :`false` _newlocalvar_1 :`true` _returnvalue_2)) :!label _label)
    (if (< _returnvalue_2 _large)
      (set `local.NewLocalVar_1` _returnvalue_2)
      (goto _label)
      (else
        (return (`local.NewLocalVar_0`))))))

(fn `FUN_Get_Start`
  (returns (Red :type "Vector Structure") (Blue :type "Vector Structure") (RedRow :type Integer) (RedColumn :type Integer) (BlueRow :type Integer) (BlueColumn :type Integer))
  (bind _cubeconfig (`self.CubeConfig`))
  (bind _returnvalue (/ (`self.CubeHeight`) 2.0))
  (bind _output (`|GetArrayItem` (`self.Cubes`) (`KismetArrayLibrary.Array_Find` _cubeconfig "NewEnumerator1")))
  (bind _output_2 (`|GetArrayItem` (`self.Cubes`) (`KismetArrayLibrary.Array_Find` _cubeconfig "NewEnumerator0")))
  (return (+ (`SceneComponent.K2_GetComponentLocation` _output_2) (`KismetMathLibrary.MakeVector` 0.0 0.0 _returnvalue)) (+ (`SceneComponent.K2_GetComponentLocation` _output) (`KismetMathLibrary.MakeVector` 0.0 0.0 _returnvalue)) (`/Game/Top/BP/Coms_Cube.IndexRow` _output_2) (`/Game/Top/BP/Coms_Cube.IndexColumn` _output_2) (`/Game/Top/BP/Coms_Cube.IndexRow` _output) (`/Game/Top/BP/Coms_Cube.IndexColumn` _output)))

(fn `FUN_Modify_Cube`
  (params (Index :type Integer) (CubeType :type "/Game/Top/BP/Variable/Enum_CubeType Enum" :default "NewEnumerator2"))
  (bind _com (`self.FUN_Get_Com_ByIndex` Index))
  (set `/Game/Top/BP/Coms_Cube.CubeType` CubeType _com)
  (`StaticMeshComponent.SetStaticMesh` _com (`BlueprintMapLibrary.Map_Find` (`self.CubeMeshConfig`) CubeType)))

(fn `FUN_Show_Target`
  (params (bNewVisibility :type Boolean) (NewLocation :type "Vector Structure"))
  (bind _target (`self.Target`))
  (`SceneComponent.SetVisibility` _target true false)
  (`SceneComponent.K2_SetWorldLocation` _target (+ NewLocation (0.0 0.0 6.0)) false false)
  (`MeshComponent.SetVectorParameterValueOnMaterials` _target "BaseColor" (`KismetMathLibrary.SelectVector` (0.0 1.0 0.0) (1.0 0.0 0.0) bNewVisibility)))

(fn `FUN_SpawnButton`
  (locals (Local :type "Array of SceneComponent Object Reference"))
  (bind _output_get (set `local.Local` (`SceneComponent.GetChildrenComponents` (`self.Com_Button`) true)))
  (for _array_element _output_get
    (`ActorComponent.K2_DestroyComponent` _array_element))
  (for _array_element_2 (`self.Button`)
    (bind (_index _id _text _mesh) (break `/Game/Top/BP/Variable/Str_Button` _array_element_2))
    (bind (_com _isvalid) (`self.FUN_Get_Com_ByIndex` _index))
    (if _isvalid
      (bind _returnvalue (`AddComponent|NODE_AddComs_Button-0` :`bManualAttachment` true :`Level` self :`Index` _index :`ID` _id))
      (`StaticMeshComponent.SetStaticMesh` _returnvalue _mesh)
      (`SceneComponent.K2_AttachToComponent` _returnvalue (`self.Com_Button`) "None" "KeepRelative" "KeepRelative" "KeepRelative" true)
      (bind _returnvalue_2 (+ (`SceneComponent.K2_GetComponentLocation` _com) (`KismetMathLibrary.MakeVector` 0.0 0.0 (+ (/ (`self.CubeHeight`) 2.0) 10.0))))
      (`SceneComponent.K2_SetWorldLocationAndRotation` :`self` _returnvalue :`NewLocation` _returnvalue_2)
      (if (not (`KismetTextLibrary.TextIsEmpty` _text))
        (bind _returnvalue_3 (`AddComponent|NODE_AddTextRenderComponent-2` :`bManualAttachment` true))
        (`SceneComponent.K2_AttachToComponent` _returnvalue_3 (`self.Com_Button`) "None" "KeepRelative" "KeepRelative" "KeepRelative" true)
        (`SceneComponent.K2_SetWorldLocationAndRotation` _returnvalue_3 (+ _returnvalue_2 (0.0 0.0 5.0)) (struct :`Pitch` 90.0 :`Roll` -90.0) false false)
        (`TextRenderComponent.K2_SetText` _returnvalue_3 _text)))))

(fn `FUN_SpawnCube`
  (locals (Local :type "/Game/Top/BP/Variable/Enum_CubeType Enum"))
  (bind _returnvalue (* (`self.Raw`) (`self.Column`)))
  (if (< (`KismetArrayLibrary.Array_Length` (`self.CubeConfig`)) _returnvalue)
    (`KismetArrayLibrary.Array_Set` (`self.CubeConfig`) (- _returnvalue 1) "NewEnumerator2" true))
  (if (>= (`KismetArrayLibrary.Array_Length` (`self.CubeConfig`)) (* (`self.Raw`) (`self.Column`)))
    (`self.FUN_ClearCube`)
    (for _index (range (`self.Raw`))
      (for _index_2 (range (`self.Column`))
        (bind _returnvalue_2 (+ (* _index (`self.Column`)) _index_2))
        (bind _output (`|GetArrayItem` (`self.CubeConfig`) _returnvalue_2))
        (bind _output_get (set `local.Local` (select `bool` (`|EnumEquality` _output "NewEnumerator2") :`false` _output :`true` (select `bool` (`self.RandomNormalCube`) :`false` _output :`true` (select `int` (`KismetMathLibrary.RandomIntegerInRange` 0 2) :`0` (enumliteral `/Game/Top/BP/Variable/Enum_CubeType` "NewEnumerator3") :`1` (enumliteral `/Game/Top/BP/Variable/Enum_CubeType` "NewEnumerator4") :`2` (enumliteral `/Game/Top/BP/Variable/Enum_CubeType` "NewEnumerator2"))))))
        (bind _returnvalue_3 (`AddComponent|NODE_AddComs_Cube-0` :`bManualAttachment` true :`Level` self :`Index` _returnvalue_2 :`IndexRow` _index :`IndexColumn` _index_2 :`CubeType` _output_get))
        (`StaticMeshComponent.SetStaticMesh` _returnvalue_3 (`BlueprintMapLibrary.Map_Find` (`self.CubeMeshConfig`) _output_get))
        (`SceneComponent.K2_AttachToComponent` _returnvalue_3 (`self.Com_Cubes`) "None" "KeepRelative" "KeepRelative" "KeepRelative" true)
        (bind _returnvalue_4 (* _index (`self.CubeSize`)))
        (bind _returnvalue_5 (* _index_2 (`self.CubeSize`)))
        (`SceneComponent.K2_SetRelativeLocation` _returnvalue_3 (`KismetMathLibrary.MakeVector` _returnvalue_4 _returnvalue_5) false false)
        (`KismetArrayLibrary.Array_Add` (`self.Cubes`) _returnvalue_3)
        (if (`self.ShowNum`)
          (bind _returnvalue_6 (`AddComponent|NODE_AddTextRenderComponent-0` :`bManualAttachment` true))
          (`SceneComponent.K2_AttachToComponent` _returnvalue_6 (`self.Com_Cubes`) "None" "KeepRelative" "KeepRelative" "KeepRelative" true)
          (`SceneComponent.K2_SetRelativeLocation` _returnvalue_6 (`KismetMathLibrary.MakeVector` _returnvalue_4 _returnvalue_5 (/ (`self.CubeHeight`) 1.5)) false false)
          (`TextRenderComponent.K2_SetText` _returnvalue_6 (`|FormatText` "{num}" _returnvalue_2)))))
    (else
      (`KismetSystemLibrary.PrintString` "关卡盒子配置不足"))))

(fn `FUN_SpawnDoor`
  (locals (Local :type "Array of SceneComponent Object Reference"))
  (bind _output_get (set `local.Local` (`SceneComponent.GetChildrenComponents` (`self.Com_Door`) true)))
  (for _array_element _output_get
    (`ActorComponent.K2_DestroyComponent` _array_element))
  (for _array_element_2 (`self.Door`)
    (bind _returnvalue (`|AddComponentByClass` (`.Door_22_49A7E92F4B6D49F0667BEB959CFC79D2` (break `/Game/Top/BP/Variable/Str_Door` _array_element_2)) true (struct) self _array_element_2))
    (`/Game/Top/BP/Coms_Door.FUN_Set_Location` _returnvalue)))

(fn `FUN_SpawnWall`
  (locals (Local :type "Array of SceneComponent Object Reference"))
  (bind _output_get (set `local.Local` (`SceneComponent.GetChildrenComponents` (`self.Com_Walls`) true)))
  (for _array_element _output_get
    (`ActorComponent.K2_DestroyComponent` _array_element))
  (for _array_element_2 (`self.BlockWall`)
    (bind (_a _b _spawnwall) (break `/Game/Top/BP/Variable/Str_BlockWall` _array_element_2))
    (bind _returnvalue (`KismetMathLibrary.Abs_Int` (- _a _b)))
    (bind _returnvalue_2 (== _returnvalue 1))
    (if (and _spawnwall (or _returnvalue_2 (== _returnvalue (`self.Column`))))
      (bind _returnvalue_3 (`AddComponent|NODE_AddStaticMeshComponent-0` :`bManualAttachment` true))
      (`SceneComponent.K2_AttachToComponent` _returnvalue_3 (`self.Com_Walls`) "None" "KeepRelative" "KeepRelative" "KeepRelative" true)
      (`SceneComponent.K2_SetWorldLocationAndRotation` _returnvalue_3 (+ (/ (+ (`SceneComponent.K2_GetComponentLocation` (`self.FUN_Get_Com_ByIndex` _b)) (`SceneComponent.K2_GetComponentLocation` (`self.FUN_Get_Com_ByIndex` _a))) 2) (`KismetMathLibrary.MakeVector` 0.0 0.0 (`self.CubeHeight`))) (select `bool` _returnvalue_2 :`true` (struct :`Yaw` 90.0) :!type "Rotator Structure") false false))))

(fn `UserConstructionScript`
  (`self.FUN_SpawnCube`)
  (`self.FUN_SpawnWall`)
  (`self.FUN_SpawnButton`)
  (`self.FUN_SpawnDoor`))