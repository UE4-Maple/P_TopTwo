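; Player controller for a grid-based level that lets the Key input operate doors through buttons.
; On Key press it looks up the button at the current PCH row and column from the game mode's level, then finds the door sharing that button's ID.
; If both are valid it calls the door's key event.
; A character-switch call to the game mode is present but never runs.
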(event `InputAction|Switch`
  (params (Key :type "Key Structure")))

(event `InputAction|Key`
  (params (Key :type "Key Structure"))
  (bind _asgm_main (`/Game/Top/BP/FUNL_Main.FUNL_Get_GameMode`))
  (bind (_nowrow _nowcolumn) (`/Game/Top/GamePlay/GM_Main.FUN_Get_NowPCH_Location` _asgm_main))
  (bind _bp_level (`/Game/Top/GamePlay/GM_Main.BP_Level` _asgm_main))
  (bind (_isvalid _ascoms_button) (`/Game/Top/BP/BP_Level.FUN_Get_Button_ByRow` _bp_level _nowrow _nowcolumn))
  (bind (_isvalid_2 _ascoms_door) (`/Game/Top/BP/BP_Level.FUN_Get_Door_ByID` _bp_level (`/Game/Top/BP/Coms_Button.ID` _ascoms_button)))
  (:`Pressed`
    (if _isvalid
      (if _isvalid_2
        (`/Game/Top/BP/Coms_Door.EVE_Key` _ascoms_door)))))

(fn `UserConstructionScript`)